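; Asteroid actor that acts as a hazard for the player and can be destroyed by impacts.
; Overlapping SS_Player_BP damages the player, plays an explosion effect and sound at the asteroid's location, then destroys it.
; TakeImpact works in two stages: the first hit activates an impact particle system, and the next calls OnExplosion.
; OnExplosion flags the asteroid as destroyed and removes it without spawning explosion effects.
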(event EventBeginPlay)

(event EventActorBeginOverlap
  (params (OtherActor :type Actor%20Object%20Reference))
  (bind _returnvalue (Transformation|GetActorLocation))
  (bind _asss_player_bp (Utilities|Casting|CastToSS_Player_BP OtherActor))
  (Default|TakeDamage _asss_player_bp)
  (Effects|SpawnEmitteratLocation "/Game/StarterContent/Particles/P_Explosion.P_Explosion" _returnvalue)
  (Audio|PlaySoundatLocation "/Game/StarterContent/Audio/Explosion_Cue.Explosion_Cue" _returnvalue "0, 0, 0" 1.0 1.0 0.0 0 0 0 0)
  (Actor|DestroyActor))

(event EventTick
  (params (DeltaSeconds :type Float%20%28single-precision%29))
  (|CallParentFunction DeltaSeconds))

(fn ConstructionScript
  (|CallParentFunction))

(fn TakeImpact
  (if (Variables|Default|GetIsImpacted)
    (CallFunction|OnExplosion)
    (else
      (Variables|Default|SetIsImpacted true)
      (Components|Activation|Activate (Variables|Default|GetImpact%20Particle%20System) false))))

(fn OnExplosion
  (Variables|Default|SetIsDestroyed true)
  (Actor|DestroyActor))