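; Plasma bolt actor, apparently a player projectile, that destroys whatever non-player actor it overlaps.
; On overlap it spawns an explosion emitter and sound at its location, then casts the player pawn to SS_Player_BP to call UpdateScore.
; Only if that cast succeeds are the other actor and the bolt destroyed; there is no filter on target type beyond excluding the player pawn.
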(event EventBeginPlay)

(event EventActorBeginOverlap
  (params (OtherActor :type Actor%20Object%20Reference))
  (bind _returnvalue (Transformation|GetActorLocation))
  (if (!= OtherActor (Game|Player|GetPlayerPawn 0))
    (Effects|SpawnEmitteratLocation "/Game/StarterContent/Particles/P_Explosion.P_Explosion" _returnvalue)
    (Audio|PlaySoundatLocation "/Game/StarterContent/Audio/Explosion_Cue.Explosion_Cue" _returnvalue "0, 0, 0" 1.0 1.0 0.0 0 0 0 0)
    (bind _asss_player_bp (Utilities|Casting|CastToSS_Player_BP (Game|Player|GetPlayerPawn 0)))
    (Default|UpdateScore _asss_player_bp)
    (Actor|DestroyActor OtherActor)
    (Actor|DestroyActor)))

(event EventTick
  (params (DeltaSeconds :type Float%20%28single-precision%29))
  (|CallParentFunction 0.0))

(fn ConstructionScript
  (|CallParentFunction))