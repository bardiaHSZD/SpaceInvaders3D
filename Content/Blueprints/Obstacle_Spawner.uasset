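; Obstacle spawner actor that periodically spawns either an Asteroid or a Health_Pickup at its own transform.
; BeginPlay starts a timer on the Spawn function with a random delay between SpawnTimeMin and SpawnTimeMax.
; Spawn rolls against HealthPickupProbability to choose the class and plays a matching sound, Pong for pickups and Bong for asteroids.
; It then re-arms its own one-shot timer, so each interval is freshly randomized.
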(event EventBeginPlay
  (Utilities|Time|SetTimerbyFunctionName 0 "Spawn" (Math|Random|RandomFloatinRange (Variables|Default|GetSpawn%20Time%20Min) (Variables|Default|GetSpawn%20Time%20Max))))

(event EventActorBeginOverlap
  (params (OtherActor :type Actor%20Object%20Reference)))

(event EventTick
  (params (DeltaSeconds :type Float%20%28single-precision%29)))

(fn ConstructionScript)

(fn Spawn
  (if (< (Math|Random|RandomFloat) (Variables|Default|GetHealth%20Pickup%20Probability))
    (Audio|PlaySoundatLocation "/Game/Audio/Pong.Pong" (Transformation|GetActorLocation) "0, 0, 0" 1.0 1.0 0.0 0 0 0 0)
    (Game|SpawnActorfromClass "/Game/Blueprints/Health_Pickup.Health_Pickup_C" (Transformation|GetActorTransform) "Undefined" 0 0)
    (else
      (Audio|PlaySoundatLocation "/Game/Audio/bong.bong" (Transformation|GetActorLocation) "0, 0, 0" 1.0 1.0 0.0 0 0 0 0)
      (Game|SpawnActorfromClass "/Game/Blueprints/Asteroid.Asteroid_C" (Transformation|GetActorTransform) "Undefined" 0 0)))
  (Utilities|Time|SetTimerbyFunctionName 0 "Spawn" (Math|Random|RandomFloatinRange (Variables|Default|GetSpawn%20Time%20Min) (Variables|Default|GetSpawn%20Time%20Max))))