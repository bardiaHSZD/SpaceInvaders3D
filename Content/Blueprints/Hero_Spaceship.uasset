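; Player spaceship that moves along a horizontal input axis, fires plasma bolts and tracks the score.
; It creates the HUD at BeginPlay and forwards axis input to a MoveRight function not defined here.
; Health is a two-hit flag: the first hit turns on damage particles, which healing clears, and the second triggers death.
; Death explodes and hides the ship, then a timer calls GoToMainMenu on the game mode.
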(event Custom|UpdateScore
  (Math|Float|IncrementFloat (Variables|Default|GetScore)))

(event EventBeginPlay
  (bind _returnvalue (UserInterface|CreateWidget "/Game/StartMenuGame/HereoHUD.HereoHUD_C" (Game|GetPlayerController 0)))
  (UserInterface|Viewport|AddtoViewport _returnvalue 0))

(event EventActorBeginOverlap
  (params (OtherActor :type Actor%20Object%20Reference)))

(event EventTick
  (params (DeltaSeconds :type Float%20%28single-precision%29)))

(event Input|ActionEvents|InputActionFire
  (params (Key :type Key%20Structure :default "None"))
  (:Pressed
    (if (not (Variables|Default|GetIs%20Dead))
      (Game|SpawnActorfromClass "/Game/Blueprints/Plasma_Bolt.Plasma_Bolt_C" (Transformation|GetActorTransform) "Undefined" 0 0)
      (Audio|PlaySound2D "/Game/Audio/pop.pop" 1.0 1.0 0.0 0 0))))

(event Input|AxisEvents|InputAxisMoveRight
  (params (AxisValue :type Float%20%28single-precision%29))
  (Class|DefaultPawn|MoveRight AxisValue))

(fn ConstructionScript)

(fn TakeDamage
  (if (Variables|Default|GetIs%20Damaged)
    (CallFunction|OnDeath)
    (else
      (Variables|Default|SetIs%20Damaged true)
      (Components|Activation|Activate (Variables|Default|GetDamage%20Particle%20System) false))))

(fn OnDeath
  (Effects|SpawnEmitteratLocation "/Game/StarterContent/Particles/P_Explosion.P_Explosion" (Transformation|GetActorLocation))
  (Variables|Default|SetIs%20Dead true)
  (Rendering|SetActorHiddenInGame true)
  (Collision|SetActorEnableCollision false)
  (Utilities|Time|SetTimerbyFunctionName (Game|GetGameMode) "GoToMainMenu" 3.0))

(fn HealDamage
  (Variables|Default|SetIs%20Damaged false)
  (Components|Activation|Deactivate (Variables|Default|GetDamage%20Particle%20System)))